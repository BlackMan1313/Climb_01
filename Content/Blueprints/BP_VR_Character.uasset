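; VR player character with arc-aimed teleporting and hand-over-hand climbing.
; Holding the Teleport axis predicts a projectile path from the right controller, shown by a Niagara beam and destination ring; release moves the capsule there.
; Grab spheres cache climbable actors; gripping while overlapping one switches to Flying and makes that hand the sole anchor.
; Tick offsets the pawn opposite that hand's movement, and releasing restores Falling once neither hand climbs.
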(event `InputAxis|Teleport`
  (params (AxisValue :type "Float (single-precision)"))
  (bind _motioncontrollerrightaim (`self.MotionControllerRightAim`))
  (if (> AxisValue 0.0)
    (`|ExecutionSequence`
      (:`then_0`
        (bind (_outhit _outpathpositions) (`GameplayStatics.Blueprint_PredictProjectilePath_ByObjectType` (`SceneComponent.K2_GetComponentLocation` _motioncontrollerrightaim) (* (`SceneComponent.GetForwardVector` _motioncontrollerrightaim) (`KismetMathLibrary.Conv_DoubleToVector` 650.0)) true 3.0 (`|MakeArray` "ObjectTypeQuery1" :!type "EObjectTypeQuery Enum")))
        (bind _output_get (set `self.PathPoints` _outpathpositions))
        (`KismetArrayLibrary.Array_Insert` _output_get (`SceneComponent.K2_GetComponentLocation` (`self.MotionControllerRight`)))
        (bind (_bblockinghit _binitialoverlap _time _distance _location _impactpoint _normal) (`GameplayStatics.BreakHitResult` _outhit))
        (set `self.ProjectedTeleportLocation` _location)
        (set `self.ProjectedTeleportNormal` _normal))
      (:`then_1`
        (`NiagaraDataInterfaceArrayFunctionLibrary.SetNiagaraArrayVector` (`self.NS_BeemPath`) "PathPoints" (`self.PathPoints`))
        (`ActorComponent.Activate` (`self.NS_BeemPath`) false)
        (`ActorComponent.Activate` (`self.NS_RingDestination`) false)
        (`SceneComponent.K2_SetWorldTransform` (`self.NS_RingDestination`) (`KismetMathLibrary.MakeTransform` (`self.ProjectedTeleportLocation`) (`KismetMathLibrary.MakeRotFromZ` (`self.ProjectedTeleportNormal`))) false false)
        (set `self.TraceActive` true)))
    (elif (`self.TraceActive`)
      (`ActorComponent.Deactivate` (`self.NS_BeemPath`))
      (`self.K2_SetActorLocation` (+ (* (`CapsuleComponent.GetScaledCapsuleHalfHeight` (`self.CapsuleComponent`)) (`SceneComponent.GetUpVector` (`self.CapsuleComponent`))) (`self.ProjectedTeleportLocation`)) false true)
      (`ActorComponent.Deactivate` (`self.NS_RingDestination`))
      (set `self.TraceActive` false))))

(event `InputAction|GrabLeft`
  (params (Key :type "Key Structure"))
  (:`Pressed`
    (if (`self.IsOverlappingActor` (`self.As BP Climbable Actor_L`))
      (if (`self.isClimbing_R`)
        (set `self.isClimbing_R` false))
      (set `self.ClimbingStartLocation` (`SceneComponent.K2_GetComponentLocation` (`self.MotionControllerLeft`)))
      (`CharacterMovementComponent.SetMovementMode` (`self.CharacterMovement`) "MOVE_Flying" 0)
      (set `self.isClimbing_L` true)))
  (:`Released`
    (set `self.isClimbing_L` false)
    (`self.SetFallingMode`)))

(event `InputAction|GrabRight`
  (params (Key :type "Key Structure"))
  (:`Pressed`
    (if (`self.IsOverlappingActor` (`self.As BP Climb Actor_R`))
      (if (`self.isClimbing_L`)
        (set `self.isClimbing_L` false))
      (set `self.ClimbingStartLocation` (`SceneComponent.K2_GetComponentLocation` (`self.MotionControllerRight`)))
      (`CharacterMovementComponent.SetMovementMode` (`self.CharacterMovement`) "MOVE_Flying" 0)
      (set `self.isClimbing_R` true)))
  (:`Released`
    (set `self.isClimbing_R` false)
    (`self.SetFallingMode`)))

(event `self.GrabSphere_Right.OnComponentBeginOverlap`
  (params (OverlappedComponent :type "PrimitiveComponent Object Reference") (OtherActor :type "Actor Object Reference") (OtherComp :type "PrimitiveComponent Object Reference") (OtherBodyIndex :type Integer) (bFromSweep :type Boolean) (SweepResult :type "HitResult Structure (by ref)"))
  (bind _asbp_climbable_actor (cast `/Game/Blueprints/BP_ClimbableActor` OtherActor))
  (set `self.As BP Climb Actor_R` _asbp_climbable_actor))

(event `self.GrabSphere1_Left.OnComponentBeginOverlap`
  (params (OverlappedComponent :type "PrimitiveComponent Object Reference") (OtherActor :type "Actor Object Reference") (OtherComp :type "PrimitiveComponent Object Reference") (OtherBodyIndex :type Integer) (bFromSweep :type Boolean) (SweepResult :type "HitResult Structure (by ref)"))
  (bind _asbp_climbable_actor (cast `/Game/Blueprints/BP_ClimbableActor` OtherActor))
  (set `self.As BP Climbable Actor_L` _asbp_climbable_actor))

(event `self.ReceiveTick`
  (params (DeltaSeconds :type "Float (single-precision)"))
  (`|ExecutionSequence`
    (:`then_0`
      (if (`self.isClimbing_R`)
        (`self.OffsetPawn` (`self.MotionControllerRight`))))
    (:`then_1`
      (if (`self.isClimbing_L`)
        (`self.OffsetPawn` (`self.MotionControllerLeft`))))))

(fn `OffsetPawn`
  (params (MotionController :type "MotionControllerComponent Object Reference"))
  (`self.K2_AddActorWorldOffset` (`KismetMathLibrary.NegateVector` (- (`SceneComponent.K2_GetComponentLocation` MotionController) (`self.ClimbingStartLocation`)))))

(fn `SetFallingMode`
  (if (and (not (`self.isClimbing_R`)) (not (`self.isClimbing_L`)))
    (`CharacterMovementComponent.SetMovementMode` (`self.CharacterMovement`) "MOVE_Falling" 0)))

(fn `UserConstructionScript`)